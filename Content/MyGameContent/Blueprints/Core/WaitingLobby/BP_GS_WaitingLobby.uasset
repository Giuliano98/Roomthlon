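; Game state for the waiting lobby that tracks ready players and starts the match by server travel to the gameplay level.
; On authority it hooks the lobby game mode's new-player login dispatcher to broadcast ready-player updates, as it does on each ready toggle.
; When everyone is ready, a looping timer runs a countdown, shown only by a placeholder print; a later mismatch cancels and resets it.
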(event `self.ReceiveBeginPlay`
  (`parent.ReceiveBeginPlay`)
  (`/Engine/EditorBlueprintResources/ActorMacros.Switch Has Authority`
    (:`Authority`
      (bind _asbp_gm_waiting_lobby (cast `/Game/MyGameContent/Blueprints/Core/WaitingLobby/BP_GM_WaitingLobby` (`self.AuthorityGameMode`))
        (:`then`
          (add `/Game/MyGameContent/Blueprints/Core/WaitingLobby/BP_GM_WaitingLobby.ED_NewPlayerLogIn` _asbp_gm_waiting_lobby (delegate `ED_NewPlayerLogIn_Event`)))
        (:`CastFailed`
          (`KismetSystemLibrary.PrintString` "FAIL CAST TO GAME MODE WAITTINGLOBBY" true true (struct :`R` 1.0 :`B` 0.08466 :`A` 1.0) 50.0))))))

(event `ED_NewPlayerLogIn_Event`
  (`self.ED_UpdateReadyPlayers`))

(event `/Game/MyGameContent/Blueprints/Interfaces/BPI_WaitingLobby.PlayerIsReady`
  (params (`bIsReady?` :type Boolean))
  (bind _playersready (`self.PlayersReady`))
  (if `bIsReady?`
    (`/Engine/EditorBlueprintResources/StandardMacros.IncrementInt` _playersready
      (:`  `
        _))
    (else
      (`/Engine/EditorBlueprintResources/StandardMacros.DecrementInt` _playersready
        (:`  `
          _))))
  (`self.ED_UpdateReadyPlayers`)
  (`self.CheckStartGame`))

(event `CheckStartGame`
  (if (== (`self.PlayersReady`) (`KismetArrayLibrary.Array_Length` (`self.PlayerArray`)))
    (bind _returnvalue (`KismetSystemLibrary.K2_SetTimerDelegate` (delegate `StartCountdown`) 1.0 true))
    (set `self.StartMatchTimer` _returnvalue)
    (elif (`KismetSystemLibrary.K2_IsValidTimerHandle` (`self.StartMatchTimer`))
      (`KismetSystemLibrary.K2_ClearAndInvalidateTimerHandle` (`self.StartMatchTimer`))
      (set `self.Countdown` 11))))

(event `StartCountdown`
  (bind _result (`/Engine/EditorBlueprintResources/StandardMacros.DecrementInt` (`self.Countdown`))
    (:`  `
      (`KismetSystemLibrary.PrintString` (`KismetStringLibrary.Conv_IntToString` _result)) ; CHANGE FOR SOMETHING ON THE HUD
      (if (== (`self.Countdown`) 0)
        (`KismetSystemLibrary.ExecuteConsoleCommand` (`KismetStringLibrary.Concat_StrStr` "servertravel " (`self.GameplayLevelName`)) null) ; Load Gameplay Level
      ))))

(fn `UserConstructionScript`
  (`parent.UserConstructionScript`))