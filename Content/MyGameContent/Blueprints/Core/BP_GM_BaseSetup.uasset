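; Base game mode that tracks connected player controllers and provides random-start spawning.
; Login and controller-swap events add controllers to AllPlayerControllers, and logout removes those that cast to BP_PC_BaseSetup.
; HandleStartingNewPlayer is overridden empty, suppressing default spawning.
; SpawnPlayer, not called within this Blueprint, destroys any current pawn, then spawns and possesses a BP_ThirdPersonCharacter at a random PlayerStart.
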(event `self.K2_PostLogin`
  (params (NewPlayer :type "PlayerController Object Reference"))
  ;[0 0.6953 1] Connect / Disconnect Events
  ;;[1 0.5149 0] Player Connect Event
  (`KismetArrayLibrary.Array_Add` (`self.AllPlayerControllers`) NewPlayer))

(event `self.K2_OnSwapPlayerControllers`
  (params (OldPC :type "PlayerController Object Reference") (NewPC :type "PlayerController Object Reference"))
  ;[0 0.6953 1] Connect / Disconnect Events
  ;;[1 0.5149 0] Player Connect Event
  (`KismetArrayLibrary.Array_Add` (`self.AllPlayerControllers`) NewPC))

(event `self.HandleStartingNewPlayer`
  (params (NewPlayer :type "PlayerController Object Reference")))

(event `self.K2_OnLogout`
  (params (ExitingController :type "Controller Object Reference"))
  ;[0 0.6953 1] Connect / Disconnect Events
  ;;[1 0.5149 0] Player Disconect Event
  (bind _asbp_pc_base_setup (cast `/Game/MyGameContent/Blueprints/Core/BP_PC_BaseSetup` ExitingController))
  (`KismetArrayLibrary.Array_RemoveItem` (`self.AllPlayerControllers`) _asbp_pc_base_setup))

(fn `FindRandomPlayerStart`
  (returns (PlayerStartTranform :type "Transform Structure (by ref)"))
  (bind _outactors (`GameplayStatics.GetAllActorsOfClass` "/Script/Engine.PlayerStart"))
  (return (`self.GetTransform` (`KismetArrayLibrary.Array_Random` _outactors))))

(fn `SpawnPlayer`
  (params (PlayerController :type "PlayerController Object Reference"))
  (bind _returnvalue (`Controller.K2_GetPawn` PlayerController))
  (`/Engine/EditorBlueprintResources/StandardMacros.IsValid` _returnvalue
    (:`Is Valid`
      (`self.K2_DestroyActor` _returnvalue))
    (:`Is Not Valid`
      _))
  (bind _returnvalue_2 (`|SpawnActorFromClass` "/Game/ThirdPerson/Blueprints/BP_ThirdPersonCharacter.BP_ThirdPersonCharacter_C" (`self.FindRandomPlayerStart`) "Undefined" "OverrideRootScale" null null))
  (`Controller.Possess` PlayerController _returnvalue_2))

(fn `UserConstructionScript`)