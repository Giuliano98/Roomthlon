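; BP_GS_Gameplay is the gameplay game state that tracks how many players are ready to start.
; PressedStartButton recounts PlayersReadyToStart from zero by checking the ReadyToStart flag on each BP_PS_Gameplay in PlayerArray.
; It then calls the UpdateReadyPlayers event dispatcher so listeners can react to the new count.
; BeginPlay and the construction script only call their parents.
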(event `self.ReceiveBeginPlay`
  (`parent.ReceiveBeginPlay`))

(event `/Game/MyGameContent/Blueprints/Interfaces/BPI_StartButton.PressedStartButton`
  (set `self.PlayersReadyToStart` 0)
  (for _array_element (`self.PlayerArray`)
    (bind _asbp_ps_gameplay (cast `/Game/MyGameContent/Blueprints/Core/Gameplay/BP_PS_Gameplay` _array_element))
    (if (`/Game/MyGameContent/Blueprints/Core/Gameplay/BP_PS_Gameplay.ReadyToStart?` _asbp_ps_gameplay)
      (`/Engine/EditorBlueprintResources/StandardMacros.IncrementInt` (`self.PlayersReadyToStart`))))
  (`self.ED_UpdateReadyPlayers`))

(fn `UserConstructionScript`
  (`parent.UserConstructionScript`))