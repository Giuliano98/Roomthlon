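; Spawner manager that procedurally builds a chain of randomly picked bridge and room blocks on BeginPlay.
; It alternates spawns from the bridge and room class arrays, with delays between steps and debug prints of array indices.
; The first bridge is positioned through its own ReallocatedRoom, then each new block through that of the last stored block.
; Each block joins ArrAllBlocks, and the loop repeats until the array exceeds a fixed size.
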(event `self.ReceiveBeginPlay`
  (bind _arrallblocks (`self.arrAllBlocks`))
  (bind _arrallblocks_2 (`self.arrAllBlocks`))
  (bind _arrallblocks_3 (`self.arrAllBlocks`))
  (bind _arrallblocks_4 (`self.arrAllBlocks`))
  (bind _returnvalue (`KismetArrayLibrary.Array_LastIndex` _arrallblocks_4))
  (bind _returnvalue_2 (`KismetArrayLibrary.Array_LastIndex` _arrallblocks_2))
  (`KismetArrayLibrary.Array_Clear` (`self.arrAllBlocks`))
  ;[0.7344 0 1] Comment
  (`KismetSystemLibrary.Delay` 2.0)
  (bind _returnvalue_3 (`|SpawnActorFromClass` (`KismetArrayLibrary.Array_Random` (`self.arrBridges`)) (`KismetMathLibrary.MakeTransform` (0.0 0.0 0.0)) "Undefined" "OverrideRootScale" null null))
  (`self.ReallocatedRoom` _returnvalue_3)
  (`KismetArrayLibrary.Array_Add` _arrallblocks _returnvalue_3)
  (`KismetSystemLibrary.PrintString` (`KismetStringLibrary.Conv_IntToString` (`KismetArrayLibrary.Array_LastIndex` _arrallblocks)))
  (`KismetSystemLibrary.Delay` 2.0)
  (bind _returnvalue_4 (`|SpawnActorFromClass` (`KismetArrayLibrary.Array_Random` (`self.arrRooms`)) (`KismetMathLibrary.MakeTransform` (0.0 0.0 0.0)) "Undefined" "OverrideRootScale" null null))
  (`KismetSystemLibrary.PrintString` (`KismetStringLibrary.Conv_IntToString` _returnvalue))
  (`self.ReallocatedRoom` (`|GetArrayItem` _arrallblocks_4 _returnvalue) _returnvalue_4)
  (`KismetArrayLibrary.Array_Add` (`self.arrAllBlocks`) _returnvalue_4)
  (`KismetSystemLibrary.Delay` 2.0 :!label _label)
  (bind _returnvalue_5 (`|SpawnActorFromClass` (`KismetArrayLibrary.Array_Random` (`self.arrBridges`)) (`KismetMathLibrary.MakeTransform` (0.0 0.0 0.0)) "Undefined" "OverrideRootScale" null null))
  (`self.ReallocatedRoom` (`|GetArrayItem` _arrallblocks_2 _returnvalue_2) _returnvalue_5)
  (`KismetSystemLibrary.PrintString` (`KismetStringLibrary.Conv_IntToString` _returnvalue_2))
  (`KismetArrayLibrary.Array_Add` (`self.arrAllBlocks`) _returnvalue_5)
  (`KismetSystemLibrary.Delay` 2.0)
  (bind _returnvalue_6 (`|SpawnActorFromClass` (`KismetArrayLibrary.Array_Random` (`self.arrRooms`)) (`KismetMathLibrary.MakeTransform` (0.0 0.0 0.0)) "Undefined" "OverrideRootScale" null null))
  (`KismetSystemLibrary.Delay` 1.0)
  (`self.ReallocatedRoom` (`|GetArrayItem` _arrallblocks_3 (`KismetArrayLibrary.Array_LastIndex` _arrallblocks_3)) _returnvalue_6)
  (bind _returnvalue_7 (`KismetArrayLibrary.Array_Add` (`self.arrAllBlocks`) _returnvalue_6))
  (`KismetSystemLibrary.PrintString` (`KismetStringLibrary.Conv_IntToString` _returnvalue_7))
  (if (not (> (`KismetArrayLibrary.Array_Length` (`self.arrAllBlocks`)) 22))
    (goto _label)))

(event `Not use just reference`
  ;[0.7344 0 1] Comment
)

(fn `UserConstructionScript`)