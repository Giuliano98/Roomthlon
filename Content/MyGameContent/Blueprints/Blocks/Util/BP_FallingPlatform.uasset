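; BP_FallingPlatform is a server-authoritative platform that drops shortly after a player steps on it, then respawns at its starting spot.
; On BeginPlay the authority stores the platform location and randomizes the fall and reappear delays.
; A player overlap, gated by a DoOnce, enables physics after the delay.
; Overlapping a BP_DeadZone hides it, waits, teleports it back with physics off, shows it and resets the DoOnce.
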(event `self.ReceiveBeginPlay`
  (`/Engine/EditorBlueprintResources/ActorMacros.Switch Has Authority`
    (:`Authority`
      (set `self.InitLocation` (`SceneComponent.K2_GetComponentLocation` (`self.Platform`)))
      (set `self.TimeBeforeFalling` (`KismetMathLibrary.RandomFloatInRange` 0.8 1.3))
      (set `self.TimeBeforeReappear` (`KismetMathLibrary.RandomFloatInRange` 2.0 4.0)))))

(event `self.Sphere.OnComponentBeginOverlap`
  (params (OverlappedComponent :type "PrimitiveComponent Object Reference") (OtherActor :type "Actor Object Reference") (OtherComp :type "PrimitiveComponent Object Reference") (OtherBodyIndex :type Integer) (bFromSweep :type Boolean) (SweepResult :type "HitResult Structure (by ref)"))
  (`/Engine/EditorBlueprintResources/ActorMacros.Switch Has Authority`
    (:`Authority`
      (if (`KismetSystemLibrary.DoesImplementInterface` OtherActor "/Game/MyGameContent/Blueprints/Interfaces/BPI_RequestsToPlayerCharacter.BPI_RequestsToPlayerCharacter_C")
        (`/Engine/EditorBlueprintResources/StandardMacros.DoOnce` false :!label _label
          (:`Completed`
            (`KismetSystemLibrary.Delay` (`self.TimeBeforeFalling`))
            (`PrimitiveComponent.SetSimulatePhysics` (`self.Platform`) true)))
        (else
          (cast `/Game/MyGameContent/Blueprints/Blocks/Util/BP_DeadZone` OtherActor)
          (`self.CE_SetEnableFallingPlatform` false)
          (`KismetSystemLibrary.Delay` (`self.TimeBeforeReappear`))
          (`self.CE_SetPhysics&Location`)
          (`self.CE_SetEnableFallingPlatform` true)
          (`self.CE_ResetCanSetPhysics`))))))

(event `CE_ResetCanSetPhysics`
  (goto _label :!via `Reset`))

(event `CE_SetEnableFallingPlatform`
  (params (`Enable?` :type Boolean))
  (`self.SetActorHiddenInGame` (not `Enable?`))
  (set `PrimitiveComponent.bGenerateOverlapEvents` `Enable?` (`self.Sphere`)))

(event `CE_SetPhysics&Location`
  (`PrimitiveComponent.SetSimulatePhysics` (`self.Platform`) false)
  (`SceneComponent.K2_SetWorldLocation` (`self.Platform`) (`self.InitLocation`) false true))

(fn `UserConstructionScript`)