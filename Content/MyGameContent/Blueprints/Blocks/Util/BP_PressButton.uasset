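; BP_PressButton is a button actor that lets a player change their ready status by pressing E while inside its trigger box.
; On overlap by an actor with a valid instigator controller, it requests the player controller through a message, stores it and enables input for it.
; The key press sends the ready-status message to that single stored controller, and end overlap disables input.
; The E key is hard-coded, noted as a stand-in for an Interact input.
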(event `Key|E`
  (params (Key :type "Key Structure"))
  (:`Pressed`
    (message `/Game/MyGameContent/Blueprints/Interfaces/BPI_WaitingLobby.ChangePlayerReadyStatus` (`self.PC_Ref`))))

(event `self.Box.OnComponentBeginOverlap`
  (params (OverlappedComponent :type "PrimitiveComponent Object Reference") (OtherActor :type "Actor Object Reference") (OtherComp :type "PrimitiveComponent Object Reference") (OtherBodyIndex :type Integer) (bFromSweep :type Boolean) (SweepResult :type "HitResult Structure (by ref)"))
  (`/Engine/EditorBlueprintResources/StandardMacros.IsValid` (`self.GetInstigatorController` OtherActor)
    (:`Is Valid`
      (bind _playercontroller (message `/Game/MyGameContent/Blueprints/Interfaces/BPI_RequestsToPlayerCharacter.RequestPlayerController` OtherActor))
      (bind _output_get (set `self.PC_Ref` _playercontroller))
      (`self.EnableInput` _output_get))))

(event `self.Box.OnComponentEndOverlap`
  (params (OverlappedComponent :type "PrimitiveComponent Object Reference") (OtherActor :type "Actor Object Reference") (OtherComp :type "PrimitiveComponent Object Reference") (OtherBodyIndex :type Integer))
  (`/Engine/EditorBlueprintResources/StandardMacros.IsValid` (`self.GetInstigatorController` OtherActor)
    (:`Is Valid`
      (`self.DisableInput` (`self.PC_Ref`)))))

(fn `UserConstructionScript`)