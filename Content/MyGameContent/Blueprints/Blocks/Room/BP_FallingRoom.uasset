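; BP_FallingRoom is a challenge room where players cross falling platforms to reach a finish trigger.
; On BeginPlay the server gives the dead zone the checkpoint location for relocation and spawns a three-column grid of BP_FallingPlatform actors from a holder component.
; Middle-row platforms get random stepped drops, while the first and last rows sit at fixed heights.
; Overlapping the finish trigger reports task completion to the player's controller, on the server only.
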(event OnComponentBeginOverlap(FinishTaskTrigger)
  (params (OverlappedComponent :type Primitive%20Component%20Object%20Reference) (OtherActor :type Actor%20Object%20Reference) (OtherComp :type Primitive%20Component%20Object%20Reference) (OtherBodyIndex :type Integer) (bFromSweep :type Boolean) (SweepResult :type Hit%20Result%20Structure%20%28by%20ref%29))
  (Networking|SwitchHasAuthority
    (:Authority
      (if (Utilities|DoesObjectImplementInterface OtherActor "/Game/MyGameContent/Blueprints/Interfaces/BPI_RequestsToPlayerCharacter.BPI_RequestsToPlayerCharacter_C")
        (Class|BPITaskCompletedManager|TaskCompleted(Message) (Game|GetInstigatorController OtherActor) 0 (Utilities|Array|MakeArray self))))))

(event Custom|SpawnPlatforms
  (bind _generateplatformholder (Variables|Default|GetGeneratePlatformHolder))
  (bind _returnvalue (Transformation|GetWorldLocation _generateplatformholder))
  (for _index (range 0 (Variables|Default|GetMaxRows))
    (Variables|Default|SetCurrentRowIndex _index)
    (for _index_2 (range 0 2)
      (Variables|Default|SetCurrentColumnIndex _index_2)
      (Utilities|FlowControl|Sequence
        (:then_0
          (Variables|Default|SetSpawnLocation (Math|Vector|MakeVector (|((A*B)+C) (Math|Conversions|ToFloat(Integer) (Variables|Default|GetCurrentRowIndex)) 3.2e+02 (.x _returnvalue)) (|((A*B)+C) (Math|Conversions|ToFloat(Integer) (Variables|Default|GetCurrentColumnIndex)) 3e+02 (.y _returnvalue)) (- (.z _returnvalue) 5e+01)))
          (if (Math|Integer|InRange(Integer) (Variables|Default|GetCurrentRowIndex) 1 (Variables|Default|GetMaxRows) true false)
            (Variables|Default|SetSpawnLocation (+ (Variables|Default|GetSpawnLocation) (Math|Vector|MakeVector 0.0 0.0 (* (Math|Random|RandomIntegerinRange 1 5) -50))))
            (elif (== (Variables|Default|GetCurrentRowIndex) (Variables|Default|GetMaxRows))
              (Variables|Default|SetSpawnLocation (+ (Variables|Default|GetSpawnLocation) (Math|Vector|MakeVector 0.0 0.0 -3e+02))))))
        (:then_1
          (Game|SpawnActorfromClass "/Game/MyGameContent/Blueprints/Blocks/Util/BP_FallingPlatform.BP_FallingPlatform_C" (Math|Transform|MakeTransform (Variables|Default|GetSpawnLocation) "0, 0, 0" "5.250000,5.250000,5.250000") "Undefined" 0 0))))))

(event EventBeginPlay
  (Networking|SwitchHasAuthority
    (:Authority
      (Class|BPIDeadZone|SetRelocateVariable(Message) (Variables|/Script/Engine.ChildActorComponent|GetChildActor (Variables|Default|GetDeadZone)) (Transformation|GetWorldLocation (Variables|Default|GetPlayerCheckPoints)))
      (CallFunction|SpawnPlatforms))))

(fn ConstructionScript)