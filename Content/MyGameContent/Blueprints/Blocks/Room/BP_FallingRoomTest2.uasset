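; Falling-platform room that spawns a grid of platforms and reports task completion to the player's controller.
; On BeginPlay, the server gives the child dead zone the checkpoint location as its relocation point and spawns BP_FallingPlatform actors from a spawner point.
; The grid steps downward row by row, with random height jitter on all but the first and last rows.
; A finish trigger overlap sends the server-side completion message.
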(event `SpawnPlatforms`
  (bind (_returnvalue_x _returnvalue_y _returnvalue_z) (`KismetMathLibrary.BreakVector` (`SceneComponent.K2_GetComponentLocation` (`self.PlatformSpawnerLoc`))))
  (for _index (range (+ (`self.MaxPlatformsColumn`) 1))
    (set `self.CurrentIndexColumn` _index)
    (for _index_2 (range (+ (`self.MaxPlatformsRow`) 1))
      (set `self.CurrentIndexRow` _index_2)
      (`|ExecutionSequence`
        (:`then_0`
          (set `self.PlatformLocation` (`KismetMathLibrary.MakeVector` (+ (* (`self.CurrentIndexRow`) 380) _returnvalue_x) (+ (* (`self.CurrentIndexColumn`) 340) _returnvalue_y) _returnvalue_z))
          (if (`KismetMathLibrary.InRange_IntInt` (`self.CurrentIndexRow`) 0 (`self.MaxPlatformsRow`) false false)
            (set `self.PlatformLocation` (+ (`self.PlatformLocation`) (`KismetMathLibrary.MakeVector` 0.0 0.0 (+ (* (`self.CurrentIndexRow`) -80) (* (`KismetMathLibrary.RandomIntegerInRange` -4 11) -10)))))
            (elif (not (== (`self.MaxPlatformsRow`) 0))
              (set `self.PlatformLocation` (+ (`self.PlatformLocation`) (`KismetMathLibrary.MakeVector` 0.0 0.0 (* (`self.CurrentIndexRow`) -90)))))))
        (:`then_1`
          (`|SpawnActorFromClass` "/Game/MyGameContent/Blueprints/Blocks/Util/BP_FallingPlatform.BP_FallingPlatform_C" (`KismetMathLibrary.MakeTransform` (`self.PlatformLocation`) (struct) (5.0 5.0 5.0)) "Undefined" "OverrideRootScale" null null))))))

(event `self.ReceiveBeginPlay`
  (`/Engine/EditorBlueprintResources/ActorMacros.Switch Has Authority`
    (:`Authority`
      (message `/Game/MyGameContent/Blueprints/Interfaces/BPI_DeadZone.SetRelocateVariable` (`ChildActorComponent.ChildActor` (`self.ChildActorDeadZone`)) (`SceneComponent.K2_GetComponentLocation` (`self.PlayerCheckPoints`)))
      (`self.SpawnPlatforms`))))

(event `self.FinishTaskTrigger.OnComponentBeginOverlap`
  (params (OverlappedComponent :type "PrimitiveComponent Object Reference") (OtherActor :type "Actor Object Reference") (OtherComp :type "PrimitiveComponent Object Reference") (OtherBodyIndex :type Integer) (bFromSweep :type Boolean) (SweepResult :type "HitResult Structure (by ref)"))
  (`/Engine/EditorBlueprintResources/ActorMacros.Switch Has Authority`
    (:`Authority`
      (if (`KismetSystemLibrary.DoesImplementInterface` OtherActor "/Game/MyGameContent/Blueprints/Interfaces/BPI_RequestsToPlayerCharacter.BPI_RequestsToPlayerCharacter_C")
        (message `/Game/MyGameContent/Blueprints/Interfaces/BPI_TaskCompletedManager.TaskCompleted` (`self.GetInstigatorController` OtherActor) null (`|MakeArray` self :!type "Actor Object Reference"))))))

(fn `UserConstructionScript`
  (`parent.UserConstructionScript`))