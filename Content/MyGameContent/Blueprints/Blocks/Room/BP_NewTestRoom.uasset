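; BP_NewTestRoom is a room Blueprint that populates itself with four test button actors when play begins.
; On BeginPlay, only the authority spawns a BP_TestButtonRoom at the world transform of each of the four ButtonLoc components, with the room as owner.
; The construction script only calls its parent.
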(event `self.ReceiveBeginPlay`
  (`/Engine/EditorBlueprintResources/ActorMacros.Switch Has Authority`
    (:`Authority`
      (for _array_element (`|MakeArray` (`self.ButtonLoc1`) (`self.ButtonLoc2`) (`self.ButtonLoc3`) (`self.ButtonLoc4`))
        (`|SpawnActorFromClass` "/Game/MyGameContent/Blueprints/Blocks/Room/BP_TestButtonRoom.BP_TestButtonRoom_C" (`SceneComponent.K2_GetComponentToWorld` _array_element) "Undefined" "OverrideRootScale" self null)))))

(fn `UserConstructionScript`
  (`parent.UserConstructionScript`))