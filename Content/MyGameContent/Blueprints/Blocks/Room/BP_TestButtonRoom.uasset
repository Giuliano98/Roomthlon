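; BP_TestButtonRoom is a room button that a player presses with E to report that room's task as completed.
; A box overlap enables input for the local player's controller and disables it on exit.
; A press checks that the player hasn't completed the task, then notifies the owning room, passing itself for post-completion.
; That callback clears CanBePressed, whose RepNotify creates an arrow-material instance on the mesh.
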(event `Key|E`
  (params (Key :type "Key Structure"))
  (:`Pressed`
    (if (`self.CanBePressed?`)
      (bind _return (`/Game/MyGameContent/Blueprints/Library/BPFL_CheckTaskHelper.HasPlayerCompletedTask?` (`self.PlayerControllerRef`) (`self.GetOwner`)))
      (if (not _return)
        (message `/Game/MyGameContent/Blueprints/Interfaces/BPI_TaskCompletedManager.TaskCompleted` (`self.GetOwner`) (`self.PlayerControllerRef`) (`|MakeArray` self :!type "Actor Object Reference"))))))

(event `/Game/MyGameContent/Blueprints/Interfaces/BPI_TaskCompletedManager.TaskPostCompleted`
  (params (ClientSender :type "Actor Object Reference"))
  (`self.SR_PostRoomCompleted`))

(event `SR_PostRoomCompleted`
  (set `self.CanBePressed?` false))

(event `self.Box.OnComponentBeginOverlap`
  (params (OverlappedComponent :type "PrimitiveComponent Object Reference") (OtherActor :type "Actor Object Reference") (OtherComp :type "PrimitiveComponent Object Reference") (OtherBodyIndex :type Integer) (bFromSweep :type Boolean) (SweepResult :type "HitResult Structure (by ref)"))
  (bind _returnvalue (`self.GetInstigatorController` OtherActor))
  (`/Engine/EditorBlueprintResources/StandardMacros.IsValid` _returnvalue ; PC is Server&OwningClient
    (:`Is Valid`
      (if (`Controller.IsLocalPlayerController` _returnvalue)
        (bind _playercontroller (message `/Game/MyGameContent/Blueprints/Interfaces/BPI_RequestsToPlayerCharacter.RequestPlayerController` OtherActor))
        (bind _output_get (set `self.PlayerControllerRef` _playercontroller))
        (`self.EnableInput` _output_get)))))

(event `self.Box.OnComponentEndOverlap`
  (params (OverlappedComponent :type "PrimitiveComponent Object Reference") (OtherActor :type "Actor Object Reference") (OtherComp :type "PrimitiveComponent Object Reference") (OtherBodyIndex :type Integer))
  (bind _returnvalue (`self.GetInstigatorController` OtherActor))
  (`/Engine/EditorBlueprintResources/StandardMacros.IsValid` _returnvalue ; PC is Server&OwningClient
    (:`Is Valid`
      (if (`Controller.IsLocalPlayerController` _returnvalue)
        (`self.DisableInput` (`self.PlayerControllerRef`))))))

(fn `OnRep_CanBePressed?`
  (`PrimitiveComponent.CreateDynamicMaterialInstance` (`self.StaticMesh`) 0 "/Engine/VREditor/UI/ArrowMaterial.ArrowMaterial" "None"))

(fn `RequestPlayerControllerTest`
  (returns (PlayerController :type "PlayerController Object Reference"))
  (return null))

(fn `UserConstructionScript`)