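; BP_BlockBase is a room block Blueprint that snaps a spawned room onto its own exit to chain rooms together.
; RealocatedRoom stores the room, then rotates its root from the reversed ExitArrow forward vector, offset by the negated EnterArrow relative rotation.
; It then teleport-free moves the root by the world-space gap between the two arrows, so the new room's entrance lands on this exit.
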(fn `RealocatedRoom`
  (params (RoomSpawned :type "/Game/MyGameContent/Blueprints/Rooms/BP_BlockBase Object Reference"))
  (locals (m_room :type "/Game/MyGameContent/Blueprints/Rooms/BP_BlockBase Object Reference"))
  (bind _defaultsceneroot (`/Game/MyGameContent/Blueprints/Rooms/BP_BlockBase.DefaultSceneRoot` (`local.m_room`)))
  (set `local.m_room` RoomSpawned)
  (`|ExecutionSequence`
    (:`then_0`
      (`SceneComponent.K2_SetWorldRotation` (`/Game/MyGameContent/Blueprints/Rooms/BP_BlockBase.DefaultSceneRoot` (`local.m_room`)) (`KismetMathLibrary.Conv_VectorToRotator` (* (`SceneComponent.GetForwardVector` (`self.ExitArrow`)) -1)) false false)
      (`SceneComponent.K2_AddWorldRotation` (`/Game/MyGameContent/Blueprints/Rooms/BP_BlockBase.DefaultSceneRoot` (`local.m_room`)) (* (`SceneComponent.RelativeRotation` (`/Game/MyGameContent/Blueprints/Rooms/BP_BlockBase.EnterArrow` (`local.m_room`))) -1.0) false false))
    (:`then_1`
      (`SceneComponent.K2_SetWorldLocation` _defaultsceneroot (+ (`SceneComponent.K2_GetComponentLocation` _defaultsceneroot) (- (`SceneComponent.K2_GetComponentLocation` (`self.ExitArrow`)) (`SceneComponent.K2_GetComponentLocation` (`/Game/MyGameContent/Blueprints/Rooms/BP_BlockBase.EnterArrow` (`local.m_room`))))) false false))))

(fn `UserConstructionScript`)