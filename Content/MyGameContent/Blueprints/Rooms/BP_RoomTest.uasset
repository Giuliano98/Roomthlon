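; BP_RoomTest is a test room actor with a button that opens an invisible door.
; The Box trigger enables the actor's input while BP_ThirdPersonCharacter overlaps it and disables it on exit.
; Pressing E inside works only once: it turns off InvisibleDoor's collision, gives Button a dynamic instance of ArrowMaterial and prints a debug message.
; An unconnected node chain for reversing the actor's facing never runs.
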(event `Key|E`
  (params (Key :type "Key Structure"))
  (:`Pressed`
    (`/Engine/EditorBlueprintResources/StandardMacros.DoOnce` false
      (:`Completed`
        (`PrimitiveComponent.SetCollisionEnabled` (`self.InvisibleDoor`) "NoCollision")
        (`PrimitiveComponent.CreateDynamicMaterialInstance` (`self.Button`) 0 "/Engine/VREditor/UI/ArrowMaterial.ArrowMaterial" "None")
        (`KismetSystemLibrary.PrintString` "InvisibleDoor Disable")))))

(event `self.Box.OnComponentBeginOverlap`
  (params (OverlappedComponent :type "PrimitiveComponent Object Reference") (OtherActor :type "Actor Object Reference") (OtherComp :type "PrimitiveComponent Object Reference") (OtherBodyIndex :type Integer) (bFromSweep :type Boolean) (SweepResult :type "HitResult Structure (by ref)"))
  (bind _asbp_third_person_character (cast `/Game/ThirdPerson/Blueprints/BP_ThirdPersonCharacter` OtherActor))
  (bind _asplayer_controller (cast `PlayerController` (`Pawn.GetController` _asbp_third_person_character)))
  (`self.EnableInput` _asplayer_controller))

(event `self.Box.OnComponentEndOverlap`
  (params (OverlappedComponent :type "PrimitiveComponent Object Reference") (OtherActor :type "Actor Object Reference") (OtherComp :type "PrimitiveComponent Object Reference") (OtherBodyIndex :type Integer))
  (bind _asbp_third_person_character (cast `/Game/ThirdPerson/Blueprints/BP_ThirdPersonCharacter` OtherActor))
  (bind _asplayer_controller (cast `PlayerController` (`Pawn.GetController` _asbp_third_person_character)))
  (`self.DisableInput` _asplayer_controller))

(fn `UserConstructionScript`)