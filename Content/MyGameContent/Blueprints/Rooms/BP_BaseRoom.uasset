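; BP_BaseRoom is a base room Blueprint that builds a blockout shell in its Construction Script from Length, Width, Height and TileSize.
; Each surface is a single Block instance stretched by non-uniform scale and offset in tile units.
; Only the floor, ceiling and a test front wall are wired up.
; Alternative placement chains, including a side wall, remain disconnected and never run.
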(fn `UserConstructionScript`
  (`|ExecutionSequence`
    (:`then_0`
      (`InstancedStaticMeshComponent.AddInstance` (`self.Block`) (`KismetMathLibrary.MakeTransform` (`KismetMathLibrary.MakeVector` (`KismetMathLibrary.Conv_IntToDouble` (`self.TileSize`))) (struct) (`KismetMathLibrary.MakeVector` (`KismetMathLibrary.Conv_IntToDouble` (`self.Length`)) (`KismetMathLibrary.Conv_IntToDouble` (`self.Width`)) 1.0)) false) ; Bottom
    )
    (:`then_1`
      (`InstancedStaticMeshComponent.AddInstance` (`self.Block`) (`KismetMathLibrary.MakeTransform` (`KismetMathLibrary.MakeVector` 0.0 0.0 (`KismetMathLibrary.Conv_IntToDouble` (* (- (`self.Height`) 1) (`self.TileSize`)))) (struct) (`KismetMathLibrary.MakeVector` (`KismetMathLibrary.Conv_IntToDouble` (`self.Length`)) (`KismetMathLibrary.Conv_IntToDouble` (`self.Width`)) 1.0)) false) ; Top
    )
    (:`then_2`
      (`InstancedStaticMeshComponent.AddInstance` (`self.Block`) (`KismetMathLibrary.MakeTransform` (`KismetMathLibrary.MakeVector` (/ (`KismetMathLibrary.Conv_IntToDouble` (* (`self.Length`) (`self.TileSize`))) -2.0)) (struct) (`KismetMathLibrary.MakeVector` 1.0 (`KismetMathLibrary.Conv_IntToDouble` (`self.Width`)) (`KismetMathLibrary.Conv_IntToDouble` (`self.Height`)))) false) ; fronttest
    )))