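; BP_PlayersReadyText is a text display showing how many players are ready to start out of the total player count.
; On BeginPlay it binds to the ready-players update dispatcher on BP_GS_Gameplay.
; Each update calls SR_UpdateText, which builds a "ready/total" string from the game state's ready count and PlayerArray length.
; The string's RepNotify pushes it to the TextRender component.
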(event `self.ReceiveBeginPlay`
  (bind _asbp_gs_gameplay (cast `/Game/MyGameContent/Blueprints/Core/Gameplay/BP_GS_Gameplay` (`GameplayStatics.GetGameState`)))
  (bind _output_get (set `self.GS_Ref` _asbp_gs_gameplay))
  (add `/Game/MyGameContent/Blueprints/Core/Gameplay/BP_GS_Gameplay.UpdateReadyPlayers` _output_get (delegate `UpdateReadyPlayers_Event`)))

(event `UpdateReadyPlayers_Event`
  (`self.SR_UpdateText`))

(event `SR_UpdateText`
  (bind _gs_ref (`self.GS_Ref`))
  (set `self.ReadyPlayers/MaxPlayers` (`KismetStringLibrary.Concat_StrStr` (`KismetStringLibrary.Conv_IntToString` (`/Game/MyGameContent/Blueprints/Core/Gameplay/BP_GS_Gameplay.PlayersReadyToStart` _gs_ref)) "/" (`KismetStringLibrary.Conv_IntToString` (`KismetArrayLibrary.Array_Length` (`GameStateBase.PlayerArray` _gs_ref))))))

(fn `OnRep_ReadyPlayers/MaxPlayers`
  (`TextRenderComponent.K2_SetText` (`self.TextRender`) (`KismetTextLibrary.Conv_StringToText` (`self.ReadyPlayers/MaxPlayers`))))

(fn `UserConstructionScript`)