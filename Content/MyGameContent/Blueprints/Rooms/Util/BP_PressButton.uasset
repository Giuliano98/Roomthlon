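; BP_PressButton is a room utility actor that lets the local player press a start button while standing inside its box trigger.
; Box overlap caches the local BP_PC_Gameplay controller and enables input on the actor, and leaving the box disables it.
; Pressing E then sends PressedStartButtonMessage to that controller through the BPI_StartButton interface.
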(event `Key|E`
  (params (Key :type "Key Structure"))
  (bind _pc_ref (`self.PC_Ref`))
  (:`Pressed`
    (if (`KismetSystemLibrary.DoesImplementInterface` _pc_ref "/Game/MyGameContent/Blueprints/Interfaces/BPI_StartButton.BPI_StartButton_C")
      (message `/Game/MyGameContent/Blueprints/Interfaces/BPI_StartButton.PressedStartButton` _pc_ref))))

(event `self.Box.OnComponentBeginOverlap`
  (params (OverlappedComponent :type "PrimitiveComponent Object Reference") (OtherActor :type "Actor Object Reference") (OtherComp :type "PrimitiveComponent Object Reference") (OtherBodyIndex :type Integer) (bFromSweep :type Boolean) (SweepResult :type "HitResult Structure (by ref)"))
  (bind _instigator (`Actor.Instigator` OtherActor))
  (if (`Pawn.IsLocallyControlled` _instigator)
    (`self.PC_Ref`
      (:`then`
        _)
      (:`else`
        (bind _asbp_pc_gameplay (cast `/Game/MyGameContent/Blueprints/Core/Gameplay/BP_PC_Gameplay` (`Pawn.GetController` _instigator)))
        (set `self.PC_Ref` _asbp_pc_gameplay)))
    (`self.EnableInput` (`self.PC_Ref`))))

(event `self.Box.OnComponentEndOverlap`
  (params (OverlappedComponent :type "PrimitiveComponent Object Reference") (OtherActor :type "Actor Object Reference") (OtherComp :type "PrimitiveComponent Object Reference") (OtherBodyIndex :type Integer))
  (if (`Pawn.IsLocallyControlled` (`Actor.Instigator` OtherActor))
    (`self.DisableInput` (`self.PC_Ref`))))

(fn `UserConstructionScript`)