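; Blueprint function library of room helpers for checking player task completion and computing room placement.
; HasPlayerCompletedTask gets the player's ID and the room's list of players allowed to pass through interface messages, returning whether the ID is listed, or false if either interface is missing.
; ReallocatedRooms returns the offset from an enter arrow vector to an exit arrow vector.
; MoveRoom is a stub that returns a zero vector.
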(fn `HasPlayerCompletedTask?`
  (params (ActorClientRef :type "Actor Object Reference") (Room :type "Actor Object Reference"))
  (returns (return :type Boolean))
  (locals (bReturn :type Boolean) (LocalActorClientRef :type "Actor Object Reference") (LocalRoom :type "Actor Object Reference"))
  (set `local.LocalActorClientRef` ActorClientRef)
  (set `local.LocalRoom` Room)
  (`|ExecutionSequence`
    (:`then_0`
      (if (`KismetSystemLibrary.DoesImplementInterface` (`local.LocalActorClientRef`) "/Game/MyGameContent/Blueprints/Interfaces/BPI_RequestsToPlayerCharacter.BPI_RequestsToPlayerCharacter_C")
        (if (`KismetSystemLibrary.DoesImplementInterface` (`local.LocalRoom`) "/Game/MyGameContent/Blueprints/Interfaces/BPI_RequestsToRoom.BPI_RequestsToRoom_C")
          (bind _playerid (message `/Game/MyGameContent/Blueprints/Interfaces/BPI_RequestsToPlayerCharacter.RequestPlayerID` (`local.LocalActorClientRef`)))
          (bind _listofplayerscanpass (message `/Game/MyGameContent/Blueprints/Interfaces/BPI_RequestsToRoom.GetListOfPlayersCanPass` (`local.LocalRoom`)))
          (set `local.bReturn` (`KismetArrayLibrary.Array_Contains` _listofplayerscanpass _playerid))
          (else
            (set `local.bReturn` false)))
        (else
          (set `local.bReturn` false))))
    (:`then_1`
      (return (`local.bReturn`)))))

(fn `MoveRoom`
  (params (ExitArrow :type "Vector Structure"))
  (returns (NewExitArrow :type "Vector Structure"))
  (return (0.0 0.0 0.0)))

(fn `ReallocatedRooms`
  (params (ExitArrowVec :type "Vector Structure") (EnterArrowVec :type "Vector Structure"))
  (returns (DistanceToMove :type "Vector Structure"))
  (return (- ExitArrowVec EnterArrowVec)))