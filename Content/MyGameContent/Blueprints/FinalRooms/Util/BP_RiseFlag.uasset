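; Hold-to-complete flag interaction that either completes a room task or gives a bridge boost, depending on FlagLocation.
; Box overlap enables input for the local player, limited in rooms to the assigned player ID, and end overlap disables it.
; Left click opens a Tick gate that compares key hold time to a goal set through the floor events.
; Success notifies the owner or boosts the player, then closes the gate.
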(event `self.ReceiveTick`
  (params (DeltaSeconds :type "Float (single-precision)"))
  (`/Engine/EditorBlueprintResources/StandardMacros.Gate` true :!label _label
    (:`Exit`
      (if (>= (`PlayerController.GetInputKeyTimeDown` (`self.PC ref`) (stale `InputAction|PlayerLeftClick` Key)) (`self.HoldTimeGoal`))
        (`|ExecutionSequence`
          (:`then_0`
            (switch `/Game/MyGameContent/Blueprints/Enum/EUtilLocation` (`self.FlagLocation`)
              (:`NewEnumerator0`
                (message `/Game/MyGameContent/Blueprints/Interfaces/BPI_TaskCompletedManager.TaskCompleted` (`self.GetOwner`) (`self.PC ref`) (`|MakeArray` null :!type "Actor Object Reference")))
              (:`NewEnumerator1`
                (message `/Game/MyGameContent/Blueprints/Interfaces/BPI_StatusToPlayerController.GiveBoostToPlayer` (`self.PC ref`) 2.0))))
          (:`then_1`
            (`self.CE_CloseGate`)
            (`KismetSystemLibrary.PrintString` "finish task")))))))

(event `InputAction|PlayerLeftClick`
  (params (Key :type "Key Structure"))
  (:`Pressed`
    (goto _label :!via `Open`))
  (:`Released`
    (goto _label :!via `Close`)))

(event `CE_CloseGate`
  (goto _label :!via `Close`))

(event `/Game/MyGameContent/Blueprints/Interfaces/BPI_DominationRoomHelpers.FloorEnableSetGoalClicks`
  (params (GoalClicks :type Integer))
  (set `self.HoldTimeGoal` (`KismetMathLibrary.Conv_IntToDouble` GoalClicks)))

(event `self.Box.OnComponentBeginOverlap`
  (params (OverlappedComponent :type "PrimitiveComponent Object Reference") (OtherActor :type "Actor Object Reference") (OtherComp :type "PrimitiveComponent Object Reference") (OtherBodyIndex :type Integer) (bFromSweep :type Boolean) (SweepResult :type "HitResult Structure (by ref)"))
  (bind _returnvalue (`self.GetInstigatorController` OtherActor))
  (`/Engine/EditorBlueprintResources/StandardMacros.IsValid` _returnvalue ; PC is Server&OwningClient
    (:`Is Valid`
      (if (`Controller.IsLocalPlayerController` _returnvalue)
        (bind _playercontroller (message `/Game/MyGameContent/Blueprints/Interfaces/BPI_RequestsToPlayerCharacter.RequestPlayerController` OtherActor))
        (set `self.PC ref` _playercontroller)
        (switch `/Game/MyGameContent/Blueprints/Enum/EUtilLocation` (`self.FlagLocation`)
          (:`NewEnumerator0`
            (bind _playerid (message `/Game/MyGameContent/Blueprints/Interfaces/BPI_RequestsToPlayerCharacter.RequestPlayerID` (`self.PC ref`)))
            (if (== _playerid (`self.AssignedPlayerID`))
              (`self.EnableInput` (`self.PC ref`))
              (`KismetSystemLibrary.PrintString` "eneable input")
              (else
                (`KismetSystemLibrary.PrintString` "no input"))))
          (:`NewEnumerator1`
            (`self.EnableInput` (`self.PC ref`))))))))

(event `/Game/MyGameContent/Blueprints/Interfaces/BPI_DominationRoomHelpers.FloorEnableSetAssignPlayerID`
  (params (PlayerID :type Integer))
  (set `self.AssignedPlayerID` PlayerID))

(event `self.Box.OnComponentEndOverlap`
  (params (OverlappedComponent :type "PrimitiveComponent Object Reference") (OtherActor :type "Actor Object Reference") (OtherComp :type "PrimitiveComponent Object Reference") (OtherBodyIndex :type Integer))
  (bind _returnvalue (`self.GetInstigatorController` OtherActor))
  (`/Engine/EditorBlueprintResources/StandardMacros.IsValid` _returnvalue ; PC is Server&OwningClient
    (:`Is Valid`
      (if (`Controller.IsLocalPlayerController` _returnvalue)
        (`self.DisableInput` (`self.PC ref`))))))

(fn `OnRep_FlagLocation`)

(fn `UserConstructionScript`)