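; BP_SpawnerRoomsTEST is a test spawner that builds a short chain of random rooms capped by an end line.
; On BeginPlay, only on the authority, it picks two rooms at random from its room class array.
; Each spawned actor receives the previous exit arrow, starting from the spawner's own Arrow, and hands its ArrowExit to the next.
; BP_EndLine spawns last with the final exit arrow.
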(event `self.ReceiveBeginPlay`
  (`/Engine/EditorBlueprintResources/ActorMacros.Switch Has Authority`
    (:`Authority`
      (set `self.TempArrow` (`self.Arrow`))
      (for _ (range 2)
        (bind _returnvalue (`|SpawnActorFromClass` (`KismetArrayLibrary.Array_Random` (`self.arrRooms`)) (`KismetMathLibrary.MakeTransform` (0.0 0.0 0.0)) "Undefined" "OverrideRootScale" null (`self.TempArrow`) null))
        (set `self.TempArrow` (`/Game/MyGameContent/Blueprints/FinalRooms/RoomsBP/BP_FinalBaseRoom.ArrowExit` _returnvalue)))
      (`|SpawnActorFromClass` "/Game/MyGameContent/Blueprints/FinalRooms/MultiplayerUtil/BP_EndLine.BP_EndLine_C" (`KismetMathLibrary.MakeTransform` (0.0 0.0 0.0)) "Undefined" "OverrideRootScale" null (`self.TempArrow`) null))))

(fn `UserConstructionScript`)