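; Floor tile actor that turns left-clicks into a click challenge while the local player stands on it.
; Overlapping its box enables input, in Room mode only for the assigned player ID and with a looping timer that resets the count.
; Reaching the click goal sends task completion to the owner in Room mode or boosts the player on Bridge.
; Replicated FloorLocation also selects the floor material.
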(event `InputAction|PlayerLeftClick`
  (params (Key :type "Key Structure"))
  (:`Pressed`
    (bind _result (`/Engine/EditorBlueprintResources/StandardMacros.IncrementInt` (`self.CurrentClick`))
      (:`  `
        (if (== _result (`self.ClicksGoal`))
          (switch `/Game/MyGameContent/Blueprints/Enum/EUtilLocation` (`self.FloorLocation`)
            (:`NewEnumerator0`
              (message `/Game/MyGameContent/Blueprints/Interfaces/BPI_TaskCompletedManager.TaskCompleted` (`self.GetOwner`) (`self.PC ref`) (`|MakeArray` null :!type "Actor Object Reference")))
            (:`NewEnumerator1`
              (message `/Game/MyGameContent/Blueprints/Interfaces/BPI_StatusToPlayerController.GiveBoostToPlayer` (`self.PC ref`) 2.0))))))))

(event `self.Box(EnablePlayerInput).OnComponentBeginOverlap`
  (params (OverlappedComponent :type "PrimitiveComponent Object Reference") (OtherActor :type "Actor Object Reference") (OtherComp :type "PrimitiveComponent Object Reference") (OtherBodyIndex :type Integer) (bFromSweep :type Boolean) (SweepResult :type "HitResult Structure (by ref)"))
  (bind _returnvalue (`self.GetInstigatorController` OtherActor))
  (`/Engine/EditorBlueprintResources/StandardMacros.IsValid` _returnvalue ; PC is Server&OwningClient
    (:`Is Valid`
      (if (`Controller.IsLocalPlayerController` _returnvalue)
        (bind _playercontroller (message `/Game/MyGameContent/Blueprints/Interfaces/BPI_RequestsToPlayerCharacter.RequestPlayerController` OtherActor))
        (set `self.PC ref` _playercontroller)
        (switch `/Game/MyGameContent/Blueprints/Enum/EUtilLocation` (`self.FloorLocation`)
          (:`NewEnumerator0`
            (bind _playerid (message `/Game/MyGameContent/Blueprints/Interfaces/BPI_RequestsToPlayerCharacter.RequestPlayerID` (`self.PC ref`)))
            (if (== _playerid (`self.AssignPlayerID`))
              (`self.EnableInput` (`self.PC ref`))
              (bind _returnvalue_2 (`KismetSystemLibrary.K2_SetTimerDelegate` (delegate `CE_ResetClicks`) 6.0 true))
              (set `self.ResetClicksTimer` _returnvalue_2)))
          (:`NewEnumerator1`
            (`self.EnableInput` (`self.PC ref`))))))))

(event `CE_ResetClicks`
  (set `self.CurrentClick` 0)
  (`KismetSystemLibrary.PrintString` "clicks reset"))

(event `self.Box(EnablePlayerInput).OnComponentEndOverlap`
  (params (OverlappedComponent :type "PrimitiveComponent Object Reference") (OtherActor :type "Actor Object Reference") (OtherComp :type "PrimitiveComponent Object Reference") (OtherBodyIndex :type Integer))
  (bind _returnvalue (`self.GetInstigatorController` OtherActor))
  (`/Engine/EditorBlueprintResources/StandardMacros.IsValid` _returnvalue ; PC is Server&OwningClient
    (:`Is Valid`
      (if (`Controller.IsLocalPlayerController` _returnvalue)
        (`self.DisableInput` (`self.PC ref`))
        (set `self.CurrentClick` 0)
        (if (`KismetSystemLibrary.K2_IsValidTimerHandle` (`self.ResetClicksTimer`))
          (`KismetSystemLibrary.K2_ClearAndInvalidateTimerHandle` (`self.ResetClicksTimer`)))))))

(fn `OnRep_FloorLocation`
  (locals (NewMaterialInstance :type "MaterialInstanceDynamic Object Reference"))
  (`|ExecutionSequence`
    (:`then_0`
      (switch `/Game/MyGameContent/Blueprints/Enum/EUtilLocation` (`self.FloorLocation`)
        (:`NewEnumerator2`
          (bind _returnvalue (`PrimitiveComponent.CreateDynamicMaterialInstance` (`self.StaticMesh`) 0 "/Game/PolygonPrototype/Materials/Alts/Mat_PolygonPrototype_06.Mat_PolygonPrototype_06" "None"))
          (set `local.NewMaterialInstance` _returnvalue))
        (:`NewEnumerator0`
          (bind _returnvalue_2 (`PrimitiveComponent.CreateDynamicMaterialInstance` (`self.StaticMesh`) 0 "/Game/PolygonPrototype/Materials/Mat_PolygonPrototype_01.Mat_PolygonPrototype_01" "None"))
          (set `local.NewMaterialInstance` _returnvalue_2))
        (:`NewEnumerator1`
          (bind _returnvalue_3 (`PrimitiveComponent.CreateDynamicMaterialInstance` (`self.StaticMesh`) 0 "/Game/PolygonPrototype/Materials/Alts/Mat_PolygonPrototype_02.Mat_PolygonPrototype_02" "None"))
          (set `local.NewMaterialInstance` _returnvalue_3))))
    (:`then_1`
      (`PrimitiveComponent.SetMaterial` (`self.StaticMesh`) 0 (`local.NewMaterialInstance`)))))

(fn `UserConstructionScript`
  (locals (NewMaterialInstance :type "MaterialInstanceDynamic Object Reference"))
  (`|ExecutionSequence`
    (:`then_0`
      (switch `/Game/MyGameContent/Blueprints/Enum/EUtilLocation` (`self.FloorLocation`)
        (:`NewEnumerator2`
          (bind _returnvalue (`PrimitiveComponent.CreateDynamicMaterialInstance` (`self.StaticMesh`) 0 "/Game/PolygonPrototype/Materials/Alts/Mat_PolygonPrototype_06.Mat_PolygonPrototype_06" "None"))
          (set `local.NewMaterialInstance` _returnvalue))
        (:`NewEnumerator0`
          (bind _returnvalue_2 (`PrimitiveComponent.CreateDynamicMaterialInstance` (`self.StaticMesh`) 0 "/Game/PolygonPrototype/Materials/Mat_PolygonPrototype_01.Mat_PolygonPrototype_01" "None"))
          (set `local.NewMaterialInstance` _returnvalue_2))
        (:`NewEnumerator1`
          (bind _returnvalue_3 (`PrimitiveComponent.CreateDynamicMaterialInstance` (`self.StaticMesh`) 0 "/Game/PolygonPrototype/Materials/Alts/Mat_PolygonPrototype_02.Mat_PolygonPrototype_02" "None"))
          (set `local.NewMaterialInstance` _returnvalue_3))))
    (:`then_1`
      (`PrimitiveComponent.SetMaterial` (`self.StaticMesh`) 0 (`local.NewMaterialInstance`)))))