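; BP_BoostSlowPlatform is a platform actor that is set up as a boost or slow-down variant through the BoostSlowDown setting.
; Its construction script creates a dynamic material instance from a different prototype material for each variant, with a fallback for other values, and applies it to the instanced bar meshes.
; The slow-down variant also rotates its static mesh 90 degrees.
; This graph handles only appearance, with no speed-changing logic.
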(fn `UserConstructionScript`
  (locals (NewMaterialInstance :type "MaterialInstanceDynamic Object Reference"))
  (`|ExecutionSequence`
    (:`then_0`
      (switch `/Game/MyGameContent/Blueprints/Enum/EBoostOrSlow` (`self.Boost/SlowDown`)
        (:`NewEnumerator2`
          (bind _returnvalue (`PrimitiveComponent.CreateDynamicMaterialInstance` (`self.InstancedStaticMesh_Bars`) 0 "/Game/PolygonPrototype/Materials/Mat_PolygonPrototype_01.Mat_PolygonPrototype_01" "None"))
          (set `local.NewMaterialInstance` _returnvalue))
        (:`NewEnumerator0`
          (bind _returnvalue_2 (`PrimitiveComponent.CreateDynamicMaterialInstance` (`self.InstancedStaticMesh_Bars`) 0 "/Game/PolygonPrototype/Materials/Alts/Mat_PolygonPrototype_02.Mat_PolygonPrototype_02" "None"))
          (set `local.NewMaterialInstance` _returnvalue_2))
        (:`NewEnumerator1`
          (bind _returnvalue_3 (`PrimitiveComponent.CreateDynamicMaterialInstance` (`self.InstancedStaticMesh_Bars`) 0 "/Game/PolygonPrototype/Materials/Alts/Mat_PolygonPrototype_04.Mat_PolygonPrototype_04" "None"))
          (set `local.NewMaterialInstance` _returnvalue_3)
          (`SceneComponent.K2_SetRelativeRotation` (`self.StaticMesh`) (struct :`Yaw` 90.0) false false))))
    (:`then_1`
      (`PrimitiveComponent.SetMaterial` (`self.InstancedStaticMesh_Bars`) 0 (`local.NewMaterialInstance`)))))