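; Multiplayer trigger box that changes a player's collision response while overlapping, if that player's ID is on its can-pass list.
; Overlaps act only for a locally controlled instigator, switching the response on at entry and off at exit via messages to the player.
; TaskCompleted appends this actor to the post-completion array and forwards it to the client actor.
; TaskPostCompleted, noted as server-run, adds the sender's ID to the list.
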(event `self.BoxTrigger.OnComponentBeginOverlap`
  (params (OverlappedComponent :type "PrimitiveComponent Object Reference") (OtherActor :type "Actor Object Reference") (OtherComp :type "PrimitiveComponent Object Reference") (OtherBodyIndex :type Integer) (bFromSweep :type Boolean) (SweepResult :type "HitResult Structure (by ref)"))
  (bind _returnvalue (`self.GetInstigatorController` OtherActor))
  (`/Engine/EditorBlueprintResources/StandardMacros.IsValid` _returnvalue ; PC is Server&OwningClient
    (:`Is Valid`
      (if (`Controller.IsLocalPlayerController` _returnvalue)
        (bind _output_get (set `self.PlayerRef` OtherActor)) ; Ref Overlaped Player
        (bind _playerid (message `/Game/MyGameContent/Blueprints/Interfaces/BPI_RequestsToPlayerCharacter.RequestPlayerID` _output_get))
        (if (`KismetArrayLibrary.Array_Contains` (`self.arrCanPassPlayers`) _playerid)
          (message `/Game/MyGameContent/Blueprints/Interfaces/BPI_RequestsToPlayerCharacter.ChangeCollisionResponse` (`self.PlayerRef`) true))))))

(event `self.BoxTrigger.OnComponentEndOverlap`
  (params (OverlappedComponent :type "PrimitiveComponent Object Reference") (OtherActor :type "Actor Object Reference") (OtherComp :type "PrimitiveComponent Object Reference") (OtherBodyIndex :type Integer))
  (bind _returnvalue (`self.GetInstigatorController` OtherActor))
  (`/Engine/EditorBlueprintResources/StandardMacros.IsValid` _returnvalue ; PC is Server&OwningClient
    (:`Is Valid`
      (if (`Controller.IsLocalPlayerController` _returnvalue)
        (message `/Game/MyGameContent/Blueprints/Interfaces/BPI_RequestsToPlayerCharacter.ChangeCollisionResponse` (`self.PlayerRef`) false)))))

(event `/Game/MyGameContent/Blueprints/Interfaces/BPI_TaskCompletedManager.TaskCompleted`
  (params (ActorClientRef :type "Actor Object Reference") (arrPostCompletedActors :type "Array of Actor Object Reference (by ref)"))
  (bind _output_get (set `self.ArrPostCompletedActors` arrPostCompletedActors))
  (`KismetArrayLibrary.Array_Add` _output_get self)
  (message `/Game/MyGameContent/Blueprints/Interfaces/BPI_TaskCompletedManager.TaskCompleted` ActorClientRef null (`self.ArrPostCompletedActors`)))

(event `/Game/MyGameContent/Blueprints/Interfaces/BPI_TaskCompletedManager.TaskPostCompleted`
  (params (ClientSender :type "Actor Object Reference"))
  (bind _playerid (message `/Game/MyGameContent/Blueprints/Interfaces/BPI_RequestsToPlayerCharacter.RequestPlayerID` ClientSender))
  (if (not (`KismetArrayLibrary.Array_Contains` (`self.arrCanPassPlayers`) _playerid))
    (`KismetArrayLibrary.Array_Add` (`self.arrCanPassPlayers`) _playerid)))

(fn `GetListOfPlayersCanPass`
  (returns (ListOfPlayersCanPass :type "Array of Integer"))
  (return (`self.arrCanPassPlayers`)))

(fn `UserConstructionScript`)