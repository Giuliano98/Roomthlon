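; BP_EndLine is a multiplayer finish-line trigger that declares the first player to reach it the winner of the run.
; Its box overlap runs only on the authority and uses a SomeoneWin flag to accept a single winner.
; It requests the overlapping actor's player ID, prints the win message, then after a short delay issues a servertravel console command targeting the waiting lobby level.
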(event `self.Box.OnComponentBeginOverlap`
  (params (OverlappedComponent :type "PrimitiveComponent Object Reference") (OtherActor :type "Actor Object Reference") (OtherComp :type "PrimitiveComponent Object Reference") (OtherBodyIndex :type Integer) (bFromSweep :type Boolean) (SweepResult :type "HitResult Structure (by ref)"))
  (`/Engine/EditorBlueprintResources/ActorMacros.Switch Has Authority`
    (:`Authority`
      (if (not (`self.SomeoneWin?`))
        (bind _playerid (message `/Game/MyGameContent/Blueprints/Interfaces/BPI_RequestsToPlayerCharacter.RequestPlayerID` OtherActor))
        (set `self.SomeoneWin?` true)
        (`KismetSystemLibrary.PrintString` (`KismetStringLibrary.Concat_StrStr` "Player " (`KismetStringLibrary.Conv_IntToString` _playerid) " won the Run. " "Player will return to the lobby level soon"))
        (`KismetSystemLibrary.Delay` 3.0)
        (`KismetSystemLibrary.ExecuteConsoleCommand` (`KismetStringLibrary.Concat_StrStr` "servertravel " "WaitingLobby_Level") null) ; Load Gameplay Level
      ))))

(fn `UserConstructionScript`
  (`parent.UserConstructionScript`))