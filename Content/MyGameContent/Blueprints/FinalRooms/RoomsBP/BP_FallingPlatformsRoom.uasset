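; BP_FallingPlatformsRoom is a level room that builds a descending field of falling platforms alongside boost and slow-down elements.
; On BeginPlay, the server alone points the room and bridge dead zones at their respawn spawners and spawns the two speed modifiers.
; It then spawns BP_FallingPlatform actors in a nested-loop grid, stepping each row lower and randomizing the height of inner rows while the first and last stay regular.
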(event `self.ReceiveBeginPlay`
  (`parent.ReceiveBeginPlay`)
  (`/Engine/EditorBlueprintResources/ActorMacros.Switch Has Authority`
    (:`Authority`
      (`|ExecutionSequence`
        (:`then_0`
          (message `/Game/MyGameContent/Blueprints/Interfaces/BPI_DeadZone.SetRelocateVariable` (`ChildActorComponent.ChildActor` (`self.DeadZone(Room)`)) (`SceneComponent.K2_GetComponentLocation` (`self.Spawner(Room)`))))
        (:`then_1`
          (message `/Game/MyGameContent/Blueprints/Interfaces/BPI_DeadZone.SetRelocateVariable` (`ChildActorComponent.ChildActor` (`self.DeadZone(Bridge)`)) (`SceneComponent.K2_GetComponentLocation` (`self.Spawner(Bridge)`))))
        (:`then_2`
          (`|SpawnActorFromClass` "/Game/MyGameContent/Blueprints/FinalRooms/Util/BP_BoostSlowPlatform.BP_BoostSlowPlatform_C" (`KismetMathLibrary.MakeTransform` (`SceneComponent.K2_GetComponentLocation` (`self.BoostLoc`))) "Undefined" "OverrideRootScale" null "NewEnumerator0" 2.0 null))
        (:`then_3`
          (`|SpawnActorFromClass` "/Game/MyGameContent/Blueprints/FinalRooms/Util/BP_BoostSlowPlatform.BP_BoostSlowPlatform_C" (`KismetMathLibrary.MakeTransform` (`SceneComponent.K2_GetComponentLocation` (`self.SlowDownLoc`))) "Undefined" "OverrideRootScale" null "NewEnumerator1" 1.8 null))
        (:`then_4`
          (`self.SpawnFallingPlatforms`))))))

(event `SpawnFallingPlatforms`
  (bind (_returnvalue_x _returnvalue_y _returnvalue_z) (`KismetMathLibrary.BreakVector` (`SceneComponent.K2_GetComponentLocation` (`self.FallingPlatformsLoc`))))
  ;[0 0.3672 1] Spawning falling platforms
  (for _index (range (+ (`self.MaxPlatformsColumn`) 1))
    (set `self.CurrentIndexColumn` _index)
    (for _index_2 (range (+ (`self.MaxPlatformsRow`) 1))
      (set `self.CurrentIndexRow` _index_2)
      (`|ExecutionSequence`
        (:`then_0`
          (set `self.PlatformLocation` (`KismetMathLibrary.MakeVector` (+ (* (`self.CurrentIndexRow`) 320) _returnvalue_x) (+ (* (`self.CurrentIndexColumn`) 200) _returnvalue_y) _returnvalue_z))
          (if (`KismetMathLibrary.InRange_IntInt` (`self.CurrentIndexRow`) 0 (`self.MaxPlatformsRow`) false false)
            (set `self.PlatformLocation` (+ (`self.PlatformLocation`) (`KismetMathLibrary.MakeVector` 0.0 0.0 (+ (* (`self.CurrentIndexRow`) -60) (* (`KismetMathLibrary.RandomIntegerInRange` -3 12) -10)))))
            (elif (not (== (`self.MaxPlatformsRow`) 0))
              (set `self.PlatformLocation` (+ (`self.PlatformLocation`) (`KismetMathLibrary.MakeVector` 0.0 0.0 (* (`self.CurrentIndexRow`) -60)))))))
        (:`then_1`
          (`|SpawnActorFromClass` "/Game/MyGameContent/Blueprints/Blocks/Util/BP_FallingPlatform.BP_FallingPlatform_C" (`KismetMathLibrary.MakeTransform` (`self.PlatformLocation`) (struct) (3.0 3.0 3.0)) "Undefined" "OverrideRootScale" null null))))))

(fn `UserConstructionScript`
  (`parent.UserConstructionScript`))