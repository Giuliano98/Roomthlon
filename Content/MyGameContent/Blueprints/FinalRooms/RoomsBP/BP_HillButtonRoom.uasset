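; Hill button room Blueprint that gives each entering player their own rise flag and relays task completion.
; On BeginPlay the server spawns four BP_RiseFlag actors at fixed points, each with a lower hold-time goal by index.
; A server-side trigger overlap hands flags out in entry order, once per player ID, so earlier entrants get longer holds.
; TaskCompleted forwards completion to the BoxTriggerCollision child actor.
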(event OnComponentBeginOverlap(BoxTrigger)
  (params (OverlappedComponent :type Primitive%20Component%20Object%20Reference) (OtherActor :type Actor%20Object%20Reference) (OtherComp :type Primitive%20Component%20Object%20Reference) (OtherBodyIndex :type Integer) (bFromSweep :type Boolean) (SweepResult :type Hit%20Result%20Structure%20%28by%20ref%29))
  (Networking|SwitchHasAuthority
    (:Authority
      (bind _playerid (Class|BPIRequeststoPlayerCharacter|RequestPlayerID(Message) OtherActor))
      (bind _output_get (Variables|Default|SetEnteredPlayerID _playerid))
      (if (not (Utilities|Set|Contains (Variables|Default|GetPlayersEntered) _output_get))
        (Utilities|FlowControl|Sequence
          (:then_0
            (Class|BPIDominationRoomHelpers|FloorEnableSetAssignPlayerID(Message) (Utilities|Array|Get(acopy) (Variables|Default|GetarrRiseFlags) (Utilities|Set|Length (Variables|Default|GetPlayersEntered))) (Variables|Default|GetEnteredPlayerID)))
          (:then_1
            (Utilities|Set|Add (Variables|Default|GetPlayersEntered) (Variables|Default|GetEnteredPlayerID))))))))

(event EventBeginPlay
  (|CallParentFunction)
  (Networking|SwitchHasAuthority
    (:Authority
      (Utilities|Array|Clear (Variables|Default|GetarrRiseFlags))
      (for (_array_element _array_index) (Utilities|Array|MakeArray (Variables|Default|GetFlagPos1) (Variables|Default|GetFlagPos2) (Variables|Default|GetFlagPos3) (Variables|Default|GetFlagPos4))
        (bind _returnvalue (Game|SpawnActorfromClass "/Game/MyGameContent/Blueprints/FinalRooms/Util/BP_RiseFlag.BP_RiseFlag_C" (Transformation|GetWorldTransform _array_element) "Undefined" self (|(8-(A*1.200000)) _array_index) "NewEnumerator0" 0))
        (Utilities|Array|Add (Variables|Default|GetarrRiseFlags) _returnvalue)))))

(event EventTaskCompleted
  (params (ActorClientRef :type Actor%20Object%20Reference) (arrPostCompletedActors :type Array%20of%20Actor%20Object%20References))
  (Class|BPITaskCompletedManager|TaskCompleted(Message) (Variables|/Script/Engine.ChildActorComponent|GetChildActor (Variables|Default|GetBoxTriggerCollision)) ActorClientRef arrPostCompletedActors)
  (Development|PrintString "task completed on roomBP"))

(fn ConstructionScript
  (|CallParentFunction))