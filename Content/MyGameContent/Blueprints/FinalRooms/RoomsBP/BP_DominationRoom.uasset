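; Domination room Blueprint that assigns each entering player, up to four, their own floor-enable child actor with a click goal.
; On the server, it owns the four floor actors and uses an overlap trigger to record unique player IDs in entry order.
; Earlier entrants get equal or higher click goals than later ones.
; Task completion is forwarded by message to the TriggerCollision child actor.
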(event `self.ReceiveBeginPlay`
  (`parent.ReceiveBeginPlay`)
  (`/Engine/EditorBlueprintResources/ActorMacros.Switch Has Authority`
    (:`Authority`
      (for _array_element (`|MakeArray` (`ChildActorComponent.ChildActor` (`self.FloorEnable1(Room)`)) (`ChildActorComponent.ChildActor` (`self.FloorEnable2(Room)`)) (`ChildActorComponent.ChildActor` (`self.FloorEnable3(Room)`)) (`ChildActorComponent.ChildActor` (`self.FloorEnable4(Room)`)))
        (`self.SetOwner` _array_element self)))))

(event `self.BoxTrigger(PlayerEnter).OnComponentBeginOverlap`
  (params (OverlappedComponent :type "PrimitiveComponent Object Reference") (OtherActor :type "Actor Object Reference") (OtherComp :type "PrimitiveComponent Object Reference") (OtherBodyIndex :type Integer) (bFromSweep :type Boolean) (SweepResult :type "HitResult Structure (by ref)"))
  (bind _enteredplayerid (`self.EnteredPlayerID`))
  (bind _childactor (`ChildActorComponent.ChildActor` (`self.FloorEnable1(Room)`)))
  (bind _childactor_2 (`ChildActorComponent.ChildActor` (`self.FloorEnable2(Room)`)))
  (bind _childactor_3 (`ChildActorComponent.ChildActor` (`self.FloorEnable3(Room)`)))
  (bind _childactor_4 (`ChildActorComponent.ChildActor` (`self.FloorEnable4(Room)`)))
  (`/Engine/EditorBlueprintResources/ActorMacros.Switch Has Authority`
    (:`Authority`
      (bind _playerid (message `/Game/MyGameContent/Blueprints/Interfaces/BPI_RequestsToPlayerCharacter.RequestPlayerID` OtherActor))
      (bind _output_get (set `self.EnteredPlayerID` _playerid))
      (if (not (`BlueprintSetLibrary.Set_Contains` (`self.PlayersEntered`) _output_get))
        (`|ExecutionSequence`
          (:`then_0`
            (switch `int` (`BlueprintSetLibrary.Set_Length` (`self.PlayersEntered`))
              (:`0`
                (message `/Game/MyGameContent/Blueprints/Interfaces/BPI_DominationRoomHelpers.FloorEnableSetAssignPlayerID` _childactor (`self.EnteredPlayerID`))
                (message `/Game/MyGameContent/Blueprints/Interfaces/BPI_DominationRoomHelpers.FloorEnableSetGoalClicks` _childactor 30))
              (:`1`
                (message `/Game/MyGameContent/Blueprints/Interfaces/BPI_DominationRoomHelpers.FloorEnableSetAssignPlayerID` _childactor_2 (`self.EnteredPlayerID`))
                (message `/Game/MyGameContent/Blueprints/Interfaces/BPI_DominationRoomHelpers.FloorEnableSetGoalClicks` _childactor_2 25))
              (:`2`
                (message `/Game/MyGameContent/Blueprints/Interfaces/BPI_DominationRoomHelpers.FloorEnableSetAssignPlayerID` _childactor_3 (`self.EnteredPlayerID`))
                (message `/Game/MyGameContent/Blueprints/Interfaces/BPI_DominationRoomHelpers.FloorEnableSetGoalClicks` _childactor_3 20))
              (:`3`
                (message `/Game/MyGameContent/Blueprints/Interfaces/BPI_DominationRoomHelpers.FloorEnableSetAssignPlayerID` _childactor_4 (`self.EnteredPlayerID`))
                (message `/Game/MyGameContent/Blueprints/Interfaces/BPI_DominationRoomHelpers.FloorEnableSetGoalClicks` _childactor_4 20))))
          (:`then_1`
            (`BlueprintSetLibrary.Set_Add` (`self.PlayersEntered`) _enteredplayerid)
            (`KismetSystemLibrary.PrintString` (`KismetStringLibrary.Concat_StrStr` "playerID add: " (`KismetStringLibrary.Conv_IntToString` _enteredplayerid)))))))))

(event `/Game/MyGameContent/Blueprints/Interfaces/BPI_TaskCompletedManager.TaskCompleted`
  (params (ActorClientRef :type "Actor Object Reference") (arrPostCompletedActors :type "Array of Actor Object Reference (by ref)"))
  (message `/Game/MyGameContent/Blueprints/Interfaces/BPI_TaskCompletedManager.TaskCompleted` (`ChildActorComponent.ChildActor` (`self.TriggerCollision`)) ActorClientRef arrPostCompletedActors)
  (`KismetSystemLibrary.PrintString` "task completed on roomBP"))

(fn `UserConstructionScript`
  (`parent.UserConstructionScript`))