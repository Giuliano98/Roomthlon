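; BP_TestNRDoor is a test Blueprint for a networked door meant to let permitted players pass through.
; After BeginPlay, the server maps each PlayerId to false in PlayerIDPass, then sets all to true following a delay.
; End overlap checks that map for locally controlled players and resets their collision response through interface messages.
; Begin overlap only prints debug text; the logic assigning ActorPlayerRef and enabling pass-through is disconnected.
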(event `self.ReceiveBeginPlay`
  (`KismetSystemLibrary.Delay` 2.0)
  (`/Engine/EditorBlueprintResources/ActorMacros.Switch Has Authority`
    (:`Authority`
      (for _array_element (`GameStateBase.PlayerArray` (`GameplayStatics.GetGameState`))
        (`BlueprintMapLibrary.Map_Add` (`self.PlayerID/Pass`) (`PlayerState.PlayerId` _array_element)))
      (`KismetSystemLibrary.PrintString` (`KismetStringLibrary.Conv_IntToString` (`BlueprintMapLibrary.Map_Length` (`self.PlayerID/Pass`))))
      (`KismetSystemLibrary.Delay` 5.0)
      (`KismetSystemLibrary.PrintString` "All player can pass")
      (for _array_element_2 (`GameStateBase.PlayerArray` (`GameplayStatics.GetGameState`))
        (`BlueprintMapLibrary.Map_Add` (`self.PlayerID/Pass`) (`PlayerState.PlayerId` _array_element_2) true)))))

(event `CustomEvent`
  (`KismetSystemLibrary.PrintString` "Hello"))

(event `self.Box.OnComponentBeginOverlap`
  (params (OverlappedComponent :type "PrimitiveComponent Object Reference") (OtherActor :type "Actor Object Reference") (OtherComp :type "PrimitiveComponent Object Reference") (OtherBodyIndex :type Integer) (bFromSweep :type Boolean) (SweepResult :type "HitResult Structure (by ref)"))
  (`/Engine/EditorBlueprintResources/ActorMacros.Switch Has Authority`
    (:`Authority`
      (`KismetSystemLibrary.PrintString` "au"))
    (:`Remote`
      (`self.CustomEvent`))))

(event `self.Box.OnComponentEndOverlap`
  (params (OverlappedComponent :type "PrimitiveComponent Object Reference") (OtherActor :type "Actor Object Reference") (OtherComp :type "PrimitiveComponent Object Reference") (OtherBodyIndex :type Integer))
  (if (`Pawn.IsLocallyControlled` (`Actor.Instigator` OtherActor))
    (bind _playerid (message `/Game/MyGameContent/Blueprints/Interfaces/BPI_InvisibleDoor.GetOverlapedPlayerID` (`self.ActorPlayerRef`))) ; Gets the ID
    (if (`BlueprintMapLibrary.Map_Find` (`self.PlayerID/Pass`) _playerid)
      (message `/Game/MyGameContent/Blueprints/Interfaces/BPI_InvisibleDoor.ChangePlayerCollisionResponse` (`self.ActorPlayerRef`) false))))

(fn `UserConstructionScript`)